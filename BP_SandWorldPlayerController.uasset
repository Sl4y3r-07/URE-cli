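; Player controller for SandWorld that creates the base UI and HUD and bridges the game to a Pixel Streaming web frontend.
; On BeginPlay it pushes a placeholder chat message and binds frontend input, parsing JSON via VaRest to store the username.
; Debug-style number keys send responses back to the frontend to join a hardcoded voice room as JSON or mute and unmute the mic as plain strings.
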(event Custom|MessageReceivedFromPixelFrontend
  (params (Descriptor :type String))
  (bind _returnvalue (Utilities|String|MakeLiteralString "type"))
  (bind _returnvalue_2 (Class|VaRestSubsystem|DecodeJsonObject (|VaRestSubsystem) Descriptor))
  (if (Class|VaRestJsonObject|HasField _returnvalue_2 _returnvalue)
    (if (Utilities|Enum|Equal(Enum) (Class|VaRestJsonObject|GetStringField _returnvalue_2 _returnvalue) "setUsername")
      (Variables|Default|SetUsername (Class|VaRestJsonObject|GetStringField _returnvalue_2 "payload")))))

(event EventBeginPlay
  (bind _returnvalue (UserInterface|CreateWidget "/Game/UI/UI_Base.UI_Base_C" self))
  (bind _output_get (Variables|Default|SetUI%20Base _returnvalue))
  (UserInterface|Viewport|AddtoViewport _output_get 0)
  (Default|PushHUD _output_get "/Game/UI/UI_HUD.UI_HUD_C")
  (Class|SandWorldPlayerController|PushChatMessage "John Doe" "Hello")
  (EventDispatchers|AssignOnInputEvent (Variables|Default|GetPixelStreamingInput) (delegate Custom|MessageReceivedFromPixelFrontend)))

(event EventTick
  (params (DeltaSeconds :type Float%20%28single-precision%29)))

(event Input|KeyboardEvents|9
  (params (Key :type Key%20Structure :default "None"))
  ;[1 1 1] Join voice room
  (:Pressed
    (Development|PrintString "Hello")
    (bind _returnvalue (Class|VaRestSubsystem|ConstructVaRestJsonObject (|VaRestSubsystem)))
    (Class|VaRestJsonObject|SetStringField _returnvalue "roomCode" "CustomTeamGroup")
    (Class|PixelStreamingInput|SendPixelStreamingResponse (Variables|Default|GetPixelStreamingInput) (Class|VaRestJsonObject|EncodeJsontoSingleString _returnvalue))))

(event Input|KeyboardEvents|3
  (params (Key :type Key%20Structure :default "None"))
  (:Pressed
    (Class|PixelStreamingInput|SendPixelStreamingResponse (Variables|Default|GetPixelStreamingInput) "UnmuteMic")))

(event Input|KeyboardEvents|2
  (params (Key :type Key%20Structure :default "None"))
  (:Pressed
    (Class|PixelStreamingInput|SendPixelStreamingResponse (Variables|Default|GetPixelStreamingInput) "MuteMic")))

(fn ConstructionScript)

(fn SomeFunction
  (return (Utilities|String|Append (Variables|Default|GetUsername) (Utilities|GetClassDisplayName (Variables|Default|GetCommonText)))))