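; Simple actor Blueprint with no clear gameplay purpose, wiring assorted lifecycle, damage and dispatcher calls.
; Construction destroys the actor and calls OnTakeAnyDamageEvent, Reset also destroys it, and Tick reapplies a fixed lifespan every frame.
; AnyDamage calls OnTakeAnyDamageEvent, but the binding for its ReceiveIt-calling handler never runs.
; AsyncPhysicsTick calls ReceiveIt and the empty Makefunc1, while the point-damage handler and several nodes are unused stubs.
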(event Custom|OnTakeAnyDamage_Event
  (params (DamagedActor :type Actor%20Object%20Reference) (Damage :type Float%20%28single-precision%29) (DamageType :type Damage%20Type%20Object%20Reference) (InstigatedBy :type Controller%20Object%20Reference) (DamageCauser :type Actor%20Object%20Reference))
  (Default|CallReceiveIt))

(event Custom|OnTakePointDamage_Event
  (params (DamagedActor :type Actor%20Object%20Reference) (Damage :type Float%20%28single-precision%29) (InstigatedBy :type Controller%20Object%20Reference) (HitLocation :type Vector) (FHitComponent :type Primitive%20Component%20Object%20Reference) (BoneName :type Name) (ShotFromDirection :type Vector) (DamageType :type Damage%20Type%20Object%20Reference) (DamageCauser :type Actor%20Object%20Reference)))

(event EventBeginPlay)

(event Collision|EventActorBeginOverlap
  (params (OtherActor :type Actor%20Object%20Reference)))

(event EventTick
  (params (DeltaSeconds :type Float%20%28single-precision%29))
  (Actor|SetLifeSpan 1e+02))

(event Game|Damage|EventAnyDamage
  (params (Damage :type Float%20%28single-precision%29) (DamageType :type Damage%20Type%20Object%20Reference) (InstigatedBy :type Controller%20Object%20Reference) (DamageCauser :type Actor%20Object%20Reference))
  (CallFunction|OnTakeAnyDamageEvent 0 1e+02 0 InstigatedBy))

(event EventOnReset
  (Actor|DestroyActor))

(event EventAsyncPhysicsTick
  (params (DeltaSeconds :type Float%20%28single-precision%29) (SimSeconds :type Float%20%28single-precision%29))
  (Default|CallReceiveIt)
  (CallFunction|Makefunc1))

(fn ConstructionScript
  (Actor|DestroyActor)
  (CallFunction|OnTakeAnyDamageEvent 0 0.0))

(fn Makefunc1)